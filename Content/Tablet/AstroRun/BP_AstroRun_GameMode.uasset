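; Game mode for the AstroRun runner game, handling obstacle spawning, distance scoring and game over.
; After a start delay, a timer spawns an asteroid or satellite at a fixed point, re-arming itself with a shrinking interval down to a minimum.
; Tick accumulates distance at constant speed and updates the HUD found at BeginPlay.
; GameOver stops scoring, shows the restart button and cursor, then pauses after a short delay.
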(event `self.ReceiveBeginPlay`
  (bind _foundwidgets (`WidgetBlueprintLibrary.GetAllWidgetsOfClass` "/Game/Tablet/AstroRun/WBP_AstroRun_HUD.WBP_AstroRun_HUD_C" false))
  (set `self.GameHUD` (`|GetArrayItem` _foundwidgets))
  (set `self.GameIsOver` false)
  (`KismetSystemLibrary.Delay` 5.0)
  (`/Engine/EditorBlueprintResources/StandardMacros.DoOnce` false
    (:`Completed`
      (`KismetSystemLibrary.K2_SetTimerDelegate` (delegate `SpawnRandomObstacle`) (`self.Timer`) true :!label _label))))

(event `SpawnRandomObstacle`
  (bind _timer (`self.Timer`))
  (`|SpawnActorFromClass` (select `bool` (`KismetMathLibrary.RandomBool`) :`false` "/Game/Tablet/AstroRun/BP_Satellite.BP_Satellite_C" :`true` "/Game/Tablet/AstroRun/BP_Asteroid.BP_Asteroid_C" :!type "Actor Class Reference") (`KismetMathLibrary.MakeTransform` (0.0 -700.0 -270.0) (struct :`Yaw` -90.0)) "Undefined" "OverrideRootScale" null null)
  (if (<= _timer 0.75)
    (set `self.Timer` 0.75)
    (goto _label)
    (else
      (set `self.Timer` (- _timer 0.025))
      (goto _label))))

(event `self.ReceiveTick`
  (params (DeltaSeconds :type "Float (single-precision)"))
  (if (not (`self.GameIsOver`))
    (bind _output_get (set `self.TotalDistance` (+ (`self.TotalDistance`) (* DeltaSeconds 1400.0))))
    (`/Game/Tablet/AstroRun/WBP_AstroRun_HUD.Update Distance Text` (`self.GameHUD`) (/ _output_get 100.0))))

(event `GameOver`
  (bind _gamehud (`self.GameHUD`))
  (set `self.GameIsOver` true)
  (`/Game/Tablet/AstroRun/WBP_AstroRun_HUD.Show Restart Button` _gamehud)
  (set `PlayerController.bShowMouseCursor` true (`GameplayStatics.GetPlayerController` 0))
  (`WidgetBlueprintLibrary.SetInputMode_GameAndUIEx` (`GameplayStatics.GetPlayerController` 0) _gamehud "LockAlways" false)
  (`KismetSystemLibrary.Delay` 0.75)
  (`GameplayStatics.SetGamePaused` true))

(fn `UserConstructionScript`)