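; BP_GameControl opens the tablet rocket-building UI and holds a debug check of the rocket part results.
; BeginPlay creates WBP_RocketBuildingMain with UI-only input and a visible cursor.
; The Menu input's FlipFlop repeats that creation on both branches, so it never closes the widget.
; CheckFinalResult, uncalled here, checks command module, body and main engine in nested switches, printing success or failure.
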(event `self.ReceiveBeginPlay`
  (bind _returnvalue (`GameplayStatics.GetPlayerController` 0))
  (bind _returnvalue_2 (`|CreateWidget` "/Game/Tablet/RocketBuilding/WBP_RocketBuildingMain.WBP_RocketBuildingMain_C" _returnvalue :!label _label))
  (`UserWidget.AddToViewport` _returnvalue_2 0)
  (`WidgetBlueprintLibrary.SetInputMode_UIOnlyEx` _returnvalue _returnvalue_2)
  (set `PlayerController.bShowMouseCursor` true _returnvalue))

(event `InputAction|Menu`
  (params (Key :type "Key Structure"))
  (:`Pressed`
    (`/Engine/EditorBlueprintResources/StandardMacros.FlipFlop`
      (:`A`
        (goto _label))
      (:`B`
        (goto _label)))))

(fn `CheckFinalResult`
  (switch `int` (`self.Comand Module Result`)
    (:`-1`
      (`KismetSystemLibrary.PrintString` "Fail  -1"))
    (:`0`
      (`KismetSystemLibrary.PrintString` "Success")
      (switch `int` (`self.Body Result`)
        (:`-1`
          (`KismetSystemLibrary.PrintString` "Fail -1"))
        (:`0`
          (switch `int` (`self.Main Engine Result`)
            (:`-1`
              (`KismetSystemLibrary.PrintString` "Fail -1"))
            (:`0`
              (`KismetSystemLibrary.PrintString` "Success"))
            (:`1`
              (`KismetSystemLibrary.PrintString` "Fail  +1"))))
        (:`1`
          (`KismetSystemLibrary.PrintString` "Fail  +1"))))
    (:`1`
      (`KismetSystemLibrary.PrintString` "Fail  +1"))))

(fn `UserConstructionScript`)