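; BP_MarsDatabase is an actor that toggles the habitat database UI with the H key.
; On BeginPlay it enables player input, caches the first BP_UISystem, BP_Habitat and BP_CaptureCube in the level, and hides the UI.
; A FlipFlop on H alternates DisplayUI and HideUI, which set visibility of the UI actor and habitat wireframe mesh, print a debug string, and trigger the capture cube's CaptureScene.
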(event `Key|H`
  (params (Key :type "Key Structure"))
  (:`Pressed`
    (`/Engine/EditorBlueprintResources/StandardMacros.FlipFlop`
      (:`A`
        (`self.DisplayUI`))
      (:`B`
        (`self.HideUI`)))))

(event `self.ReceiveBeginPlay`
  (`self.EnableInput` (`GameplayStatics.GetPlayerController` 0))
  (bind _outactors (`GameplayStatics.GetAllActorsOfClass` "/Game/Blueprints/BP_UISystem.BP_UISystem_C"))
  (bind _output_get (set `self.Habitat UI` (`|GetArrayItem` _outactors)))
  (`SceneComponent.SetVisibility` (`Actor.RootComponent` _output_get) false true)
  (bind _outactors_2 (`GameplayStatics.GetAllActorsOfClass` "/Game/Blueprints/BP_Habitat.BP_Habitat_C"))
  (set `self.Habitat BP` (`|GetArrayItem` _outactors_2))
  (bind _outactors_3 (`GameplayStatics.GetAllActorsOfClass` "/Game/Blueprints/BP_CaptureCube.BP_CaptureCube_C"))
  (set `self.CaptureCube` (`|GetArrayItem` _outactors_3)))

(fn `DisplayUI`
  (`SceneComponent.SetVisibility` (`Actor.RootComponent` (`self.Habitat UI`)) true true)
  (`SceneComponent.SetVisibility` (`/Game/Blueprints/BP_Habitat.SM_HabitatWireframe` (`self.Habitat BP`)) true false)
  (`KismetSystemLibrary.PrintString` "On")
  (`/Game/Blueprints/BP_CaptureCube.CaptureScene` (`self.CaptureCube`)))

(fn `HideUI`
  (`SceneComponent.SetVisibility` (`Actor.RootComponent` (`self.Habitat UI`)) false true)
  (`SceneComponent.SetVisibility` (`/Game/Blueprints/BP_Habitat.SM_HabitatWireframe` (`self.Habitat BP`)) false false)
  (`KismetSystemLibrary.PrintString` "Off")
  (`/Game/Blueprints/BP_CaptureCube.CaptureScene` (`self.CaptureCube`)))

(fn `UserConstructionScript`)