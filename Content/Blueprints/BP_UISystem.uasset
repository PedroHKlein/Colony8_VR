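; BP_UISystem is an actor that places a UI widget component around its root, tuned through distance, yaw, pitch, height and scale variables.
; Its construction script sets the spring arm's length, negated pitch and yaw, and height above the root, then scales the widget on Y and Z only.
; An unconnected alternative positions without the spring arm, using vector rotation around Z and a debug limit cylinder.
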(fn `UserConstructionScript`
  (bind _springarm (`self.SpringArm`))
  (bind (_returnvalue_x _returnvalue_y _returnvalue_z) (`KismetMathLibrary.BreakVector` (`SceneComponent.K2_GetComponentLocation` (`self.DefaultSceneRoot`))))
  ;[0.314 1 0.2203] Distance from camera / Y and Z Rotation / Scale/ Height
  (set `SpringArmComponent.TargetArmLength` (`self.DistanceFromCamera`) _springarm)
  (`SceneComponent.K2_SetRelativeRotation` _springarm (`KismetMathLibrary.MakeRotator` 0.0 (* (`self.Y Rotation (Pitch)`) -1.0) (* (`self.ZRotation (Yaw)`) -1.0)) false false)
  (`SceneComponent.SetRelativeScale3D` (`self.Widget`) (* (0.0 1.0 1.0) (`self.Scale`)))
  (`SceneComponent.K2_SetWorldLocation` _springarm (`KismetMathLibrary.MakeVector` _returnvalue_x _returnvalue_y (+ _returnvalue_z (`self.Height`))) false false))