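; Controller Blueprint for the game's widgets, including a rocket simulation UI.
; On BeginPlay it shows the mouse cursor and caches the first WPP_Master and WBP_RocketSimulation widgets it finds.
; DesactivateInput overlays an empty widget on the viewport, apparently to block input, and ActivateInput calls RemoveAllWidgets to undo it.
; Widget ID cycling, UI-only input mode and the rocket result check are unconnected, so they never run.
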(event `InputAction|Next`
  (params (Key :type "Key Structure")))

(event `self.ReceiveBeginPlay`
  (set `PlayerController.bShowMouseCursor` true (`GameplayStatics.GetPlayerController` 0))
  (bind _foundwidgets (`WidgetBlueprintLibrary.GetAllWidgetsOfClass` "/Game/WPP_Master.WPP_Master_C" false))
  (set `self.Master` (`|GetArrayItem` _foundwidgets))
  (bind _foundwidgets_2 (`WidgetBlueprintLibrary.GetAllWidgetsOfClass` "/Game/RocketBuilding/WBP_RocketSimulation.WBP_RocketSimulation_C" false))
  (set `self.SimulatorWidget` (`|GetArrayItem` _foundwidgets_2)))

(fn `ActivateInput`
  (`WidgetLayoutLibrary.RemoveAllWidgets`))

(fn `DesactivateInput`
  (bind _returnvalue (`|CreateWidget` "/Game/Minigame/WPS_Empty.WPS_Empty_C"))
  (`UserWidget.AddToViewport` _returnvalue 0)
  (`KismetSystemLibrary.PrintString` "InputDisactivated"))

(fn `RocketCheckFinalResult`)

(fn `UserConstructionScript`)